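; Inventory component that holds item data assets in a slot array of InventorySize, built on BeginPlay.
; AddItem stacks onto a matching slot below the asset's max stack size, otherwise fills the first empty slot, returning true only when it stacked.
; RemoveItem finds the given entry and decrements its stack, clearing the slot at the last item.
; AddRock is a shortcut that adds the rock item asset.
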(event `self.ReceiveBeginPlay`
  (`self.InventoryConstruction`))

(fn `AddItem`
  (params (ItemToAdd :type "/Game/InventorySystem/BP_Item Object Reference"))
  (returns (HasFoundSlot1 :type Boolean))
  (locals (HasFoundSlot :type Boolean))
  (bind _hasfoundslot (`local.HasFoundSlot`))
  ;[0.3166 1 0.4028] Add Item If it already exist
  (for (_array_element _array_index) (`self.Inventory`)
    (bind (_hasitem _stucksize _itemasset) (break `/Game/InventorySystem/S_InventorySlot` _array_element))
    (if (and _hasitem (== (`local.ItemToAdd`) _itemasset) (< _stucksize (`/Game/InventorySystem/BP_Item.MaxStuckSize` (`local.ItemToAdd`))))
      (`KismetArrayLibrary.Array_Set` (`self.Inventory`) _array_index (make `/Game/InventorySystem/S_InventorySlot` true (+ _stucksize 1) (`local.ItemToAdd`)))
      (set `local.HasFoundSlot` true)
      (break)))
  (if _hasfoundslot
    (return _hasfoundslot)
    (else
      ;[1 0.03818 0] Add item if it not yet have
      (for (_array_element_2 _array_index_2) (`self.Inventory`)
        (if (not (`.HasItem_1_8E345B054AA81CE600E7EBAD864CEFBC` (break `/Game/InventorySystem/S_InventorySlot` _array_element_2)))
          (`KismetArrayLibrary.Array_Set` (`self.Inventory`) _array_index_2 (make `/Game/InventorySystem/S_InventorySlot` true 1 (`local.ItemToAdd`)))
          (set `local.HasFoundSlot` false)
          (break)))
      (return (`local.HasFoundSlot`)))))

(fn `AddRock`
  (`self.AddItem` "/Game/InventorySystem/DA_Item_Rock.DA_Item_Rock"))

(fn `InventoryConstruction`
  (`KismetArrayLibrary.Array_Clear` (`self.Inventory`))
  (for _ (range (`self.InventorySize`))
    (`KismetArrayLibrary.Array_Add` (`self.Inventory`))))

(fn `RemoveItem`
  (params (ItemToRemove :type "/Game/InventorySystem/S_InventorySlot Structure (by ref)"))
  (bind _inventory (`self.Inventory`))
  (bind _output (`|GetArrayItem` _inventory (`KismetArrayLibrary.Array_Find` _inventory ItemToRemove)))
  (bind (_hasitem _stucksize _itemasset) (break `/Game/InventorySystem/S_InventorySlot` _output))
  (if (> _stucksize 1)
    (bind _result (`/Engine/EditorBlueprintResources/StandardMacros.DecrementInt` _stucksize)
      (:`  `
        ;[1 1 1] Remove if a many items
        (`|VariableSetRef` _output (make `/Game/InventorySystem/S_InventorySlot` true _result _itemasset))))
    (else
      ;[1 1 1] Remove if one item
      (`|VariableSetRef` _output (make `/Game/InventorySystem/S_InventorySlot` false))))
  (return))