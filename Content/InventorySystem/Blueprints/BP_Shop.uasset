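; BP_Shop is an interactable shop actor that opens a shop UI backed by its own ACInventory component, which it exposes through GetInventory.
; BeginPlay creates the WBP_Shop widget once with that inventory.
; OnInteracted adds it to the viewport, refreshes its item grid, sets game-and-UI input and shows the cursor.
; A disconnected branch that would spawn stored items as world pickups and destroy the actor never runs.
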(event `self.ReceiveBeginPlay`
  (bind _returnvalue (`|CreateWidget` "/Game/InventorySystem/Widgets/WBP_Shop.WBP_Shop_C" null (`self.AC_Inventory`)))
  (set `self.ShopUi` _returnvalue))

(fn `GetInventory`
  (returns (Inventory :type "/Game/InventorySystem/Blueprints/AC_Inventory Object Reference"))
  (return (`self.AC_Inventory`)))

(fn `OnInteracted`
  (params (InteractedActor :type "Actor Object Reference"))
  (returns (InteractionFinished :type Boolean))
  (bind _returnvalue (`GameplayStatics.GetPlayerController` 0))
  (bind _shopui (`self.ShopUi`))
  (`UserWidget.AddToViewport` _shopui 0)
  (`/Game/InventorySystem/Widgets/WBP_Shop.UpdateItemsGrid` _shopui)
  (`WidgetBlueprintLibrary.SetInputMode_GameAndUIEx` _returnvalue _shopui)
  (set `PlayerController.bShowMouseCursor` true _returnvalue)
  (return false))

(fn `UserConstructionScript`)