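; BP_WorldItem is an item placed in the world that goes into the interacting actor's inventory.
; Its construction script sets the static mesh from the assigned ItemDataAsset.
; OnInteracted fetches that actor's inventory by interface message and adds one item, decrementing StackSize on success and destroying itself when the stack runs out.
; Its own GetInventory returns nothing, and the event graph is unused.
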(fn `GetInventory`
  (returns (Inventory :type "/Game/InventorySystem/Blueprints/AC_Inventory Object Reference"))
  (return null))

(fn `OnInteracted`
  (params (InteractedActor :type "Actor Object Reference"))
  (returns (InteractionFinished :type Boolean))
  (bind _inventory (message `/Game/InventorySystem/Blueprints/BPI_Interaction.GetInventory` InteractedActor))
  (`/Engine/EditorBlueprintResources/StandardMacros.IsValid` _inventory
    (:`Is Valid`
      (bind _hasfoundslot1 (`/Game/InventorySystem/Blueprints/AC_Inventory.AddItem` _inventory (`self.ItemDataAsset`)))
      (if _hasfoundslot1
        (bind _result (`/Engine/EditorBlueprintResources/StandardMacros.DecrementInt` (`self.StackSize`))
          (:`  `
            (if (<= _result 0)
              (`self.K2_DestroyActor`)))))
      (return _hasfoundslot1))))

(fn `UserConstructionScript`
  (bind _itemdataasset (`self.ItemDataAsset`))
  (`/Engine/EditorBlueprintResources/StandardMacros.IsValid` _itemdataasset
    (:`Is Valid`
      (`StaticMeshComponent.SetStaticMesh` (`self.StaticMesh`) (`/Game/InventorySystem/Data/BP_Item.Mesh` _itemdataasset)))))