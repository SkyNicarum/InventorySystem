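; Inventory component that stores items in a slot array of SInventorySlot structs, each holding an item data asset, stack count and index.
; Adding fills a matching non-full stack before taking an empty slot, while other functions remove, swap, split and merge stacks.
; Merging respects the item's max stack size and handles the source differently for left-button versus other drags.
; Mutations fire OnInventoryChanged, and AddItemDev inserts a test dynamite item.
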(event `self.ReceiveBeginPlay`)

(fn `AddItem`
  (params (ItemToAdd :type "/Game/InventorySystem/Data/BP_Item Object Reference"))
  (returns (HasFoundSlot1 :type Boolean))
  (locals (HasFoundSlot :type Boolean))
  (bind _hasfoundslot (`local.HasFoundSlot`))
  ;[0.3166 1 0.4028] Add Item If it already exist
  (for (_array_element _array_index) (`self.Inventory`)
    (bind (_hasitem _stucksize _itemasset) (break `/Game/InventorySystem/Data/S_InventorySlot` _array_element))
    (if (and _hasitem (== (`local.ItemToAdd`) _itemasset) (< _stucksize (`/Game/InventorySystem/Data/BP_Item.MaxStuckSize` (`local.ItemToAdd`))))
      (`KismetArrayLibrary.Array_Set` (`self.Inventory`) _array_index (make `/Game/InventorySystem/Data/S_InventorySlot` true (+ _stucksize 1) (`local.ItemToAdd`)))
      (set `local.HasFoundSlot` true)
      (break)))
  (if _hasfoundslot
    (`self.OnInventoryChanged`)
    (return _hasfoundslot)
    (else
      ;[1 0.03818 0] Add item if it not yet have
      (for (_array_element_2 _array_index_2) (`self.Inventory`)
        (if (not (`.HasItem_1_8E345B054AA81CE600E7EBAD864CEFBC` (break `/Game/InventorySystem/Data/S_InventorySlot` _array_element_2)))
          (`KismetArrayLibrary.Array_Set` (`self.Inventory`) _array_index_2 (make `/Game/InventorySystem/Data/S_InventorySlot` true 1 (`local.ItemToAdd`)))
          (set `local.HasFoundSlot` true)
          (break)))
      (`self.OnInventoryChanged`)
      (return (`local.HasFoundSlot`)))))

(fn `AddItemDev`
  (`self.AddItem` "/Game/InventorySystem/Data/DA_Item_DinamitTest.DA_Item_DinamitTest"))

(fn `AddItemToStack`
  (params (StackIndex :type Integer) (AmountToAdd :type Integer))
  (bind (_output_hasitem _output_stucksize _output_itemasset _output_index) (break `/Game/InventorySystem/Data/S_InventorySlot` (`|GetArrayItem` (`self.Inventory`) StackIndex)))
  (`KismetArrayLibrary.Array_Set` (`self.Inventory`) StackIndex (make `/Game/InventorySystem/Data/S_InventorySlot` _output_hasitem (+ AmountToAdd _output_stucksize) _output_itemasset _output_index))
  (`self.OnInventoryChanged`))

(fn `InventoryConstruction`
  (`KismetArrayLibrary.Array_Clear` (`self.Inventory`))
  (for _index (range (`self.InventorySize`))
    (`KismetArrayLibrary.Array_Add` (`self.Inventory`) (make `/Game/InventorySystem/Data/S_InventorySlot` false 0 null _index))))

(fn `MergeStaks`
  (params (SourceSlot :type "/Game/InventorySystem/Data/S_InventorySlot Structure") (TargetSlot :type "/Game/InventorySystem/Data/S_InventorySlot Structure") (PointerEvent :type "PointerEvent Structure"))
  (locals (Source :type "/Game/InventorySystem/Data/S_InventorySlot Structure") (Target :type "/Game/InventorySystem/Data/S_InventorySlot Structure") (Remainder :type Integer))
  (bind (_hasitem _stucksize _itemasset) (break `/Game/InventorySystem/Data/S_InventorySlot` (`local.Source`)))
  (bind (_hasitem_2 _stucksize_2 _itemasset_2) (break `/Game/InventorySystem/Data/S_InventorySlot` (`local.Source`)))
  (bind (_hasitem_3 _stucksize_3 _itemasset_3 _index) (break `/Game/InventorySystem/Data/S_InventorySlot` (`local.Target`)))
  (bind (_hasitem_4 _stucksize_4 _itemasset_4 _index_2) (break `/Game/InventorySystem/Data/S_InventorySlot` (`local.Source`)))
  (bind (_hasitem_5 _stucksize_5 _itemasset_5 _index_3) (break `/Game/InventorySystem/Data/S_InventorySlot` (`local.Target`)))
  (bind (_hasitem_6 _stucksize_6 _itemasset_6) (break `/Game/InventorySystem/Data/S_InventorySlot` (`local.Source`)))
  (bind (_hasitem_7 _stucksize_7 _itemasset_7) (break `/Game/InventorySystem/Data/S_InventorySlot` (`local.Source`)))
  (bind (_hasitem_8 _stucksize_8 _itemasset_8 _index_4) (break `/Game/InventorySystem/Data/S_InventorySlot` (`local.Target`)))
  (bind (_hasitem_9 _stucksize_9 _itemasset_9 _index_5) (break `/Game/InventorySystem/Data/S_InventorySlot` (`local.Target`)))
  (bind _returnvalue (+ _stucksize (`.StuckSize_4_53DEF0014B5240774906A38EB5DF4233` (break `/Game/InventorySystem/Data/S_InventorySlot` (`local.Target`)))))
  (bind _returnvalue_2 (+ _stucksize_7 (`.StuckSize_4_53DEF0014B5240774906A38EB5DF4233` (break `/Game/InventorySystem/Data/S_InventorySlot` (`local.Target`)))))
  (set `local.Source` SourceSlot)
  (set `local.Target` TargetSlot)
  (if (!= (`.Index_10_C202F6E64E0F3B51927D6AA35C8B1576` (break `/Game/InventorySystem/Data/S_InventorySlot` (`local.Source`))) (`.Index_10_C202F6E64E0F3B51927D6AA35C8B1576` (break `/Game/InventorySystem/Data/S_InventorySlot` (`local.Target`))))
    (if (== (`KismetInputLibrary.PointerEvent_GetEffectingButton` PointerEvent) "LeftMouseButton")
      (if (<= _returnvalue_2 (`/Game/InventorySystem/Data/BP_Item.MaxStuckSize` _itemasset_7))
        ;[1 1 1] Set Slot if target < max stack
        (`KismetArrayLibrary.Array_Set` (`self.Inventory`) _index (make `/Game/InventorySystem/Data/S_InventorySlot` _hasitem_3 _returnvalue_2 _itemasset_3 _index))
        (`KismetArrayLibrary.Array_Set` (`self.Inventory`) _index_2 (make `/Game/InventorySystem/Data/S_InventorySlot` false 0 null _index_2))
        (else
          ;[1 1 1] Set slot if target > max stack size
          (bind _output_get (set `local.Remainder` (- (+ _stucksize_6 (`.StuckSize_4_53DEF0014B5240774906A38EB5DF4233` (break `/Game/InventorySystem/Data/S_InventorySlot` (`local.Target`)))) (`/Game/InventorySystem/Data/BP_Item.MaxStuckSize` _itemasset_6))))
          (`KismetArrayLibrary.Array_Set` (`self.Inventory`) _index_3 (make `/Game/InventorySystem/Data/S_InventorySlot` _hasitem_5 (`/Game/InventorySystem/Data/BP_Item.MaxStuckSize` _itemasset_5) _itemasset_5 _index_3))
          (`self.AddItemToStack` (`.Index_10_C202F6E64E0F3B51927D6AA35C8B1576` (break `/Game/InventorySystem/Data/S_InventorySlot` (`local.Source`))) (+ (* (`.StuckSize_4_53DEF0014B5240774906A38EB5DF4233` (break `/Game/InventorySystem/Data/S_InventorySlot` (`local.Source`))) -1) (`local.Remainder`)))))
      (`self.OnInventoryChanged`)
      (else
        (if (<= _returnvalue (`/Game/InventorySystem/Data/BP_Item.MaxStuckSize` _itemasset))
          ;[1 1 1] Set Slot if target < max stack
          (`KismetArrayLibrary.Array_Set` (`self.Inventory`) _index_4 (make `/Game/InventorySystem/Data/S_InventorySlot` _hasitem_8 _returnvalue _itemasset_8 _index_4))
          (else
            (`KismetSystemLibrary.PrintString` "Down")
            ;[1 1 1] Set slot if target > max stack size
            (set `local.Remainder` (- (+ _stucksize_2 (`.StuckSize_4_53DEF0014B5240774906A38EB5DF4233` (break `/Game/InventorySystem/Data/S_InventorySlot` (`local.Target`)))) (`/Game/InventorySystem/Data/BP_Item.MaxStuckSize` _itemasset_2)))
            (`KismetArrayLibrary.Array_Set` (`self.Inventory`) _index_5 (make `/Game/InventorySystem/Data/S_InventorySlot` _hasitem_9 (`/Game/InventorySystem/Data/BP_Item.MaxStuckSize` _itemasset_9) _itemasset_9 _index_5))
            (`self.AddItemToStack` (`.Index_10_C202F6E64E0F3B51927D6AA35C8B1576` (break `/Game/InventorySystem/Data/S_InventorySlot` (`local.Source`))) (`local.Remainder`))))
        (`self.OnInventoryChanged`)))))

(fn `PutInNewStack`
  (params (InventorySlotIndex :type Integer) (Item :type "/Game/InventorySystem/Data/S_InventorySlot Structure (by ref)"))
  (`KismetArrayLibrary.Array_Set` (`self.Inventory`) InventorySlotIndex Item)
  (`self.OnInventoryChanged`))

(fn `RemoveItem`
  (params (ItemToRemove :type "/Game/InventorySystem/Data/S_InventorySlot Structure (by ref)"))
  (bind _inventory (`self.Inventory`))
  (bind _output (`|GetArrayItem` _inventory (`KismetArrayLibrary.Array_Find` _inventory ItemToRemove)))
  (bind (_hasitem _stucksize _itemasset) (break `/Game/InventorySystem/Data/S_InventorySlot` _output))
  (if (> _stucksize 1)
    (bind _result (`/Engine/EditorBlueprintResources/StandardMacros.DecrementInt` _stucksize)
      (:`  `
        ;[1 1 1] Remove if a many items
        (`|VariableSetRef` _output (make `/Game/InventorySystem/Data/S_InventorySlot` true _result _itemasset))))
    (else
      ;[1 1 1] Remove if one item
      (`|VariableSetRef` _output (make `/Game/InventorySystem/Data/S_InventorySlot` false 0 null))))
  (`self.OnInventoryChanged`)
  (return))

(fn `SplitStack`
  (params (SlotIndex :type Integer))
  (returns (SplitStack :type "/Game/InventorySystem/Data/S_InventorySlot Structure"))
  (locals (ToSubtruct :type Integer))
  (bind _output (`|GetArrayItem` (`self.Inventory`) SlotIndex))
  (bind (_hasitem _stucksize _itemasset _index) (break `/Game/InventorySystem/Data/S_InventorySlot` _output))
  (if (> _stucksize 1)
    (bind _output_get (set `local.ToSubtruct` (/ _stucksize 2)))
    (`|VariableSetRef` _output (make `/Game/InventorySystem/Data/S_InventorySlot` _hasitem (- _stucksize _output_get) _itemasset _index))
    (`self.OnInventoryChanged`)
    (return (make `/Game/InventorySystem/Data/S_InventorySlot` _hasitem (`local.ToSubtruct`) _itemasset _index))
    (else
      (`self.OnInventoryChanged`)
      (return (make `/Game/InventorySystem/Data/S_InventorySlot` false 0 null (`local.SlotIndex`))))))

(fn `SwapSlots`
  (params (IndexSource :type Integer) (IndexTarget :type Integer))
  (locals (SourceStack :type "/Game/InventorySystem/Data/S_InventorySlot Structure") (TargetStack :type "/Game/InventorySystem/Data/S_InventorySlot Structure"))
  (set `local.SourceStack` (`|GetArrayItem` (`self.Inventory`) IndexSource))
  (set `local.TargetStack` (`|GetArrayItem` (`self.Inventory`) IndexTarget))
  (`KismetArrayLibrary.Array_Set` (`self.Inventory`) (`local.IndexSource`) (`local.TargetStack`))
  (`KismetArrayLibrary.Array_Set` (`self.Inventory`) (`local.IndexTarget`) (`local.SourceStack`))
  (`self.OnInventoryChanged`))