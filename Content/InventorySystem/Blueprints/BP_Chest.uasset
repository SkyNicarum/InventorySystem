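; BP_Chest is an interactable inventory chest that shows its contents in a widget.
; On BeginPlay it creates WBP_Chest bound to its ACInventory component.
; OnInteracted adds the widget to the viewport, refreshes its item grid and switches player 0 to Game and UI input with a visible cursor.
; An unconnected branch would spawn stored items as BP_WorldItem at the Arrow and destroy the chest; GetInventory is empty.
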(event `self.ReceiveBeginPlay`
  (bind _returnvalue (`|CreateWidget` "/Game/InventorySystem/Widgets/WBP_Chest.WBP_Chest_C" null (`self.AC_Inventory`)))
  (set `self.ChestUI` _returnvalue))

(fn `GetInventory`
  (returns (Inventory :type "/Game/InventorySystem/Blueprints/AC_Inventory Object Reference"))
  (return null))

(fn `OnInteracted`
  (params (InteractedActor :type "Actor Object Reference"))
  (returns (InteractionFinished :type Boolean))
  (bind _returnvalue (`GameplayStatics.GetPlayerController` 0))
  (bind _chestui (`self.ChestUI`))
  (`UserWidget.AddToViewport` _chestui 0)
  (`/Game/InventorySystem/Widgets/WBP_Chest.UpdateItemsGrid` _chestui)
  (`WidgetBlueprintLibrary.SetInputMode_GameAndUIEx` _returnvalue _chestui)
  (set `PlayerController.bShowMouseCursor` true _returnvalue)
  (return false))

(fn `UserConstructionScript`)